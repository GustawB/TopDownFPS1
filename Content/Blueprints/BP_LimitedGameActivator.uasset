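; BP_LimitedGameActivator starts or cuts short a limited-shot game through TopDownFPS1GameModeBase, which it caches on BeginPlay.
; Tick polls IsGameActivated as a one-shot trigger, with ShouldEndFaster alternating its effect.
; One activation resets bullet-travel stats, replaces all widgets with BP_GameHUD and sets CanDoLimitedGame.
; The next sets CanDoLimitedGame again but zeroes ShotsLeft to end the game early.
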(event EventTick
  (params (DeltaSeconds :type Float%20%28single-precision%29))
  (bind _as_top_down_fps1game_mode_base (Variables|Default|GetAs%20Top%20Down%20FPS1Game%20Mode%20Base))
  (bind _as_top_down_fps1game_mode_base_2 (Variables|Default|GetAs%20Top%20Down%20FPS1Game%20Mode%20Base))
  (if (Variables|Default|GetisGameActivated)
    (if (Variables|Default|GetshouldEndFaster)
      (Variables|Default|SetshouldEndFaster false)
      (Variables|/Script/TopDownFPS1.TopDownFPS1GameModeBase|SetcanDoLimitedGame _as_top_down_fps1game_mode_base true)
      (Variables|Default|SetisGameActivated false)
      (Variables|/Script/TopDownFPS1.TopDownFPS1GameModeBase|SetshotsLeft _as_top_down_fps1game_mode_base 0.0)
      (else
        (Variables|/Script/TopDownFPS1.TopDownFPS1GameModeBase|SetMaxHowMuchBulletTravelled _as_top_down_fps1game_mode_base_2 0.0)
        (Variables|/Script/TopDownFPS1.TopDownFPS1GameModeBase|SetHowMuchBulletTravelled _as_top_down_fps1game_mode_base_2 0.0)
        (Viewport|RemoveAllWidgets)
        (bind _returnvalue (UserInterface|CreateWidget "/Game/Blueprints/BP_GameHUD.BP_GameHUD_C" (Game|GetPlayerController 0)))
        (UserInterface|Viewport|AddtoViewport _returnvalue 0)
        (Variables|/Script/TopDownFPS1.TopDownFPS1GameModeBase|SetcanDoLimitedGame (Variables|Default|GetAs%20Top%20Down%20FPS1Game%20Mode%20Base) true)
        (Variables|Default|SetisGameActivated false)
        (Variables|Default|SetshouldEndFaster true)))))

(event EventBeginPlay
  (bind _astop_down_fps1game_mode_base (Utilities|Casting|CastToTopDownFPS1GameModeBase (Game|GetGameMode)))
  (Variables|Default|SetAs%20Top%20Down%20FPS1Game%20Mode%20Base _astop_down_fps1game_mode_base))

(fn ConstructionScript)